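; BP_HealthPickUp is a spinning health pickup that the player collects by overlapping it.
; On overlap it casts to BP_FPSController and, only when Health is below MaxHealth, calls the player's HealthPickUp event, plays a sound and particle effect, then destroys itself.
; Tick applies a fixed, frame-rate-dependent yaw step and plays a timeline whose track feeds a local position offset for animation.
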(event Collision|EventActorBeginOverlap
  (params (OtherActor :type Actor%20Object%20Reference))
  (bind _cube (Variables|Default|GetCube))
  (bind _returnvalue (Transformation|GetWorldLocation _cube))
  ;[1 1 1] If player and health less than maxHealth then call the custom event function on the player to set the health and then come back here to be destroyed
  (bind _asbp_fpscontroller (Utilities|Casting|CastToBP_FPSController OtherActor))
  (if (< (Variables|/Game/Blueprints/BP_FPSController.BP_FPSController_C|GetHealth _asbp_fpscontroller) (Variables|/Game/Blueprints/BP_FPSController.BP_FPSController_C|GetMaxHealth _asbp_fpscontroller))
    (Default|HealthPickUp _asbp_fpscontroller)
    (Audio|PlaySoundatLocation "/Game/SoundEffects/PickupSound.PickupSound" _returnvalue)
    (Effects|SpawnEmitteratLocation "/Game/Particles/p_PickUp.p_PickUp" _returnvalue)
    (Actor|DestroyActor)))

(event EventTick
  (params (DeltaSeconds :type Float%20%28single-precision%29))
  ;[1 1 1] Animation
  (Transformation|AddActorLocalRotation "0,1.750000, 0" false false)
  (bind _newtrack_0 (Timeline|Timeline_0 Play)
    (:Update
      (Transformation|AddActorLocalOffset _newtrack_0 false false))))

(fn ConstructionScript)