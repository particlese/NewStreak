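; Base Blueprint for firing weapons, handling ammo, fire feedback and reloading.
; OnFire checks ammo and durability, then decrements clamped ammo and spawns a particle flash and sound at the mesh's muzzle socket.
; It has no hit or projectile logic, leaving the crosshair input unused.
; Reload refills ammo instantly with a 2D sound; no-ammo sound and reload animation are empty functions, and debug prints remain.
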(event Custom|OnFire
  (params (CrosshairWorldSpace :type Vector))
  (bind _canfire (CallFunction|CanWeaponFire))
  (bind _output_get (Variables|Default|SetCanFire? _canfire))
  (if _output_get
    (CallFunction|DecrementAmmoCount)
    (CallFunction|PlayMuzzleFlash)
    (CallFunction|PlayFireSound)
    (else
      (CallFunction|PlayNoAmmoSound)
      (Development|PrintString (Utilities|String|ToString(Boolean) _output_get)))))

(event EventBeginPlay)

(event Collision|EventActorBeginOverlap
  (params (OtherActor :type Actor%20Object%20Reference)))

(event EventTick
  (params (DeltaSeconds :type Float%20%28single-precision%29)))

(fn ConstructionScript)

(fn CanWeaponFire
  (if (> (Variables|Default|GetAmmoCount) 0.0)
    (if (> (Variables|Default|GetDurability) 0.0)
      (return true)
      (else
        _)))
  (return false))

(fn DecrementAmmoCount
  (bind _output_get (Variables|Default|SetAmmoCount (Math|Float|Clamp(Float) (- (Variables|Default|GetAmmoCount) 1.0) 0.0 (Variables|Default|GetMaxAmmoCount))))
  (Development|PrintString (Utilities|String|BuildString(Float) "" "Ammo Count" _output_get)))

(fn PlayMuzzleFlash
  (bind _muzzlesocket (Variables|Default|GetMuzzleSocket))
  (bind _mesh (Variables|Default|GetMesh))
  (Effects|SpawnEmitteratLocation "/Game/NewStreak/3rdPartyLibrariesImports/StarterContent/Particles/P_Explosion.P_Explosion" (Transformation|GetSocketLocation _mesh _muzzlesocket) (Transformation|GetSocketRotation _mesh _muzzlesocket) "0.070000,0.070000,0.070000"))

(fn PlayFireSound
  (Audio|SpawnSoundatLocation "/Game/NewStreak/3rdPartyLibrariesImports/StarterContent/Audio/Explosion02.Explosion02" (Transformation|GetSocketLocation (Variables|Default|GetMesh self) (Variables|Default|GetMuzzleSocket))))

(fn PlayNoAmmoSound)

(fn Reload
  (CallFunction|ReloadSound)
  (CallFunction|PlayReloadAnimation)
  (Variables|Default|SetAmmoCount (Variables|Default|GetMaxAmmoCount)))

(fn ReloadSound
  (Audio|PlaySound2D "/Game/NewStreak/3rdPartyLibrariesImports/StarterContent/Audio/Collapse02.Collapse02" 0.3 1.0 1.0 0 (Game|GetPlayerCharacter 0)))

(fn PlayReloadAnimation)