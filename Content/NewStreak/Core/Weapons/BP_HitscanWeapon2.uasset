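; Hitscan weapon Blueprint that fires instant line traces and applies point damage to what they hit.
; When the parent's fire logic runs and firing is allowed, the server casts several muzzle traces toward the crosshair point, randomized within a spread cone.
; Collected hits receive damage from the current ammo type, created at BeginPlay, and spawn a small explosion emitter, also within the authority-only branch.
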(event EventBeginPlay
  (bind _returnvalue (AddComponent|AddBPBaseAmmo))
  (Variables|Default|SetCurrentAmmoType _returnvalue))

(event Collision|EventActorBeginOverlap
  (params (OtherActor :type Actor%20Object%20Reference))
  (|CallParentFunction OtherActor) ; This node is disabled and will not be called.\nDrag off pins to build functionality.
)

(event EventTick
  (params (DeltaSeconds :type Float%20%28single-precision%29))
  (|CallParentFunction DeltaSeconds) ; This node is disabled and will not be called.\nDrag off pins to build functionality.
)

(event EventOnFire
  (params (CrosshairWorldSpace :type Vector :default "0, 0, 0"))
  (|CallParentFunction CrosshairWorldSpace)
  (if (Variables|Default|GetCanFire?)
    (bind _hitoccured_ (CallFunction|DetermineHitObjects CrosshairWorldSpace))
    (if _hitoccured_
      (CallFunction|ApplyDamagetoHitActors))))

(fn ConstructionScript
  (|CallParentFunction))

(fn DetermineHitObjects
  (params (CrosshairWorldSpace :type Vector))
  (bind _mesh (Variables|Character|GetMesh))
  (bind _muzzlesocket (Variables|Default|GetMuzzleSocket))
  (bind _returnvalue (Transformation|GetSocketTransform _mesh _muzzlesocket "RTS_World"))
  (Networking|SwitchHasAuthority
    (:Authority
      (Utilities|Array|Clear (Variables|Default|GetHitResults))
      (for _index (range 1 (Variables|Default|GetTracesUsed))
        (bind (_outhit _returnvalue_2) (Collision|LineTraceByChannel (.location _returnvalue) (+ (.location _returnvalue) (Math|Vector|RotateVector (* (Class|KismetMathLibrary|RandomUnitVectorinConeinRadians "1.000000, 0, 0" (Math|Trig|DegreesToRadians (Variables|Default|GetSpread))) (Variables|Default|GetRange)) (Math|Rotator|FindLookatRotation (.location _returnvalue) CrosshairWorldSpace))) "TraceTypeQuery1" false 0 "ForDuration"))
        (bind _output_get (LocalVariables|SetObjectHit? (or _returnvalue_2 (LocalVariables|GetObjectHit?))))
        (if _output_get
          (Utilities|Array|Add (Variables|Default|GetHitResults) _outhit)))
      (return (LocalVariables|GetObjectHit?)))))

(fn ApplyDamagetoHitActors
  (bind _returnvalue (Game|GetInstigatorController))
  (Networking|SwitchHasAuthority
    (:Authority
      (for _index (range 0 (- (Utilities|Array|Length (Variables|Default|GetHitResults)) 1))
        (Game|Damage|ApplyPointDamage (.HitActor (Collision|BreakHitResult (Utilities|Array|Get(acopy) (Variables|Default|GetHitResults) _index))) (Variables|/Game/NewStreak/Core/Weapons/BP_BaseAmmo.BP_BaseAmmo_C|GetBaseDamage (Variables|Default|GetCurrentAmmoType)) (Math|Rotator|GetRotationXVector (Math|Rotator|FindLookatRotation (.Location (Collision|BreakHitResult (Utilities|Array|Get(acopy) (Variables|Default|GetHitResults) _index))) (Transformation|GetActorLocation (Pawn|GetControlledPawn _returnvalue)))) (Utilities|Array|Get(acopy) (Variables|Default|GetHitResults) _index) _returnvalue self)
        (bind _output_get (Variables|Default|SetHitLocation (.Location (Collision|BreakHitResult (Utilities|Array|Get(acopy) (Variables|Default|GetHitResults) _index)))))
        (CallFunction|PlayImpactEffects _output_get)))))

(fn PlayImpactEffects
  (params (Location :type Vector))
  (Effects|SpawnEmitteratLocation "/Game/NewStreak/3rdPartyLibrariesImports/StarterContent/Particles/P_Explosion.P_Explosion" Location (Math|Conversions|RotationFromXVector Location) "0.100000,0.100000,0.100000"))