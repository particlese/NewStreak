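; BP_FPSController is the first-person player controller that handles hero switching and spawn requests.
; It caches BP_GameInstance on BeginPlay and, on the ChangeHero input, calls that instance's ChangeCharacter with itself.
; SpawnFunc passes a chosen character class to BP_FPSGamemode's SpawnRespawnPlayer, so the game mode does the actual spawning.
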(event Custom|SpawnFunc
  (params (StartClass :type BP%20FPS%20Base%20Character%20Class%20Reference))
  ;[1 1 1] Spawning via the gamemode
  (bind _asbp_fpsgamemode (Utilities|Casting|CastToBP_FPSGamemode (Game|GetGameMode)))
  (Default|SpawnRespawnPlayer _asbp_fpsgamemode self StartClass))

(event EventBeginPlay
  ;[1 1 1] Get reference to game instance at the start of play
  (bind _asbp_game_instance (Utilities|Casting|CastToBP_GameInstance (Game|GetGameInstance)))
  (Variables|Default|SetGameInstanceRef _asbp_game_instance))

(event Input|ActionEvents|InputActionChangeHero
  (params (Key :type Key%20Structure))
  ;[1 1 1] Change character
  (:Pressed
    (Default|ChangeCharacter (Variables|Default|GetGameInstanceRef) self)))

(event Input|ActionEvents|InputActionScoreboard
  (params (Key :type Key%20Structure))
  ;[1 1 1] Scoreboard
)

(fn ConstructionScript)