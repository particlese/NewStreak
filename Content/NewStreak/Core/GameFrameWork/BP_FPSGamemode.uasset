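; FPS game mode that handles player login and spawns or respawns players as a selected character class.
; On login, the server caches all PlayerStart actors and asks BP_GameInstance to change the new player's character.
; The spawn event destroys the current pawn, spawns the chosen class at a random cached start, possesses it and switches to game-only input with the cursor hidden.
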(event Custom|SpawnRespawnPlayer
  (params (playerController :type Player%20Controller%20Object%20Reference) (SelectedCharacter :type BP%20FPS%20Base%20Character%20Class%20Reference))
  ;[1 1 1] Spawn/Respawn event
  (CallFunction|SpawnasCharacter SelectedCharacter playerController))

(event EventPostLogin
  (params (NewPlayer :type Player%20Controller%20Object%20Reference))
  ;[1 1 1] OnPostLogin event
  (Networking|SwitchHasAuthority
    (:Authority
      (bind _outactors (Actor|GetAllActorsOfClass "/Script/Engine.PlayerStart"))
      (Variables|Default|SetPlayerStartPoints _outactors)
      (bind _asbp_game_instance (Utilities|Casting|CastToBP_GameInstance (Game|GetGameInstance)))
      (Default|ChangeCharacter _asbp_game_instance NewPlayer))))

(fn ConstructionScript)

(fn SpawnasCharacter
  (params (selectedCharacter :type BP%20FPS%20Base%20Character%20Class%20Reference) (playerController :type Player%20Controller%20Object%20Reference))
  (bind _returnvalue (Pawn|GetControlledPawn playerController))
  (bind _startlocation (CallFunction|StartLocation))
  (if (Utilities|IsValid _returnvalue)
    (Actor|DestroyActor _returnvalue))
  (bind _returnvalue_2 (Game|SpawnActorfromClass selectedCharacter _startlocation "AdjustIfPossibleButAlwaysSpawn" 0 0))
  (Utilities|IsValid _returnvalue_2
    (:Is%20Valid
      (Pawn|Possess playerController _returnvalue_2)
      (Variables|/Script/Engine.PlayerController|SetbShowMouseCursor playerController false)
      (Input|SetInputModeGameOnly playerController))))

(fn StartLocation
  (bind _playerstartpoints (Variables|Default|GetPlayerStartPoints))
  (return (Transformation|GetActorTransform (Utilities|Array|Get(acopy) _playerstartpoints (Math|Random|RandomIntegerinRange 0 (- (Utilities|Array|Length _playerstartpoints) 1))))))