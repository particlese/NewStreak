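; Health pickup that heals an overlapping BP_FPSBaseCharacter that is alive and below max health, then hides until it respawns.
; Overlap starts a looping timer that retries activation until the character leaves.
; An authority switch gates the heal, hide and respawn timer.
; A timeline bobs the pack and a timer rotates it, with stand spin scaled by remaining respawn time.
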(event Custom|Event%20EndOverlapHandler
  (params (Leaving%20Actor :type Actor%20Object%20Reference))
  ;[1 1 1] server side
  (Utilities|Casting|CastToBP_FPSBaseCharacter Leaving%20Actor)
  (Utilities|Time|ClearandInvalidateTimerbyHandle (Variables|FlagsAndStuff|GetactivationChecker)))

(event Custom|TryToActivate
  ;[1 1 1] server side
  ;;[1 1 1] keep checking until endOverlap triggers
  (CallFunction|TryActivatingMe (stale Custom|Event%20BeginOverlapHandler _asbp_fpsbase_character)))

(event Custom|Event%20BeginOverlapHandler
  (params (OverlappingActor :type Actor%20Object%20Reference))
  ;[1 1 1] server side
  (bind _asbp_fpsbase_character (Utilities|Casting|CastToBP_FPSBaseCharacter OverlappingActor))
  (CallFunction|TryActivatingMe _asbp_fpsbase_character)
  ;;[1 1 1] keep checking until endOverlap triggers
  (bind _returnvalue (Utilities|Time|SetTimerbyEvent (delegate Custom|TryToActivate) (Variables|ConfigVariables|GetactivationCheckerInterval) true))
  (Variables|FlagsAndStuff|SetactivationChecker _returnvalue))

(event EventBeginPlay
  ;[1 1 1] client
  ;;[1 1 1] animation
  (bind _newtrack_0 (Timeline|Timeline_0 Play)
    (:Update
      (Transformation|AddLocalOffset (Variables|Default|GethealthPickupSmall) _newtrack_0 false false)
      (CallFunction|RotationAnimation)
      (Utilities|Time|SetTimerbyFunctionName 0 "RotationAnimation" 0.01667 true))))

(event Collision|EventActorEndOverlap
  (params (OtherActor :type Actor%20Object%20Reference))
  ;[1 1 1] client
  (CallFunction|EventEndOverlapHandler OtherActor))

(event Collision|EventActorBeginOverlap
  (params (OtherActor :type Actor%20Object%20Reference))
  ;[1 1 1] client
  (CallFunction|EventBeginOverlapHandler OtherActor))

(fn ConstructionScript)

(fn RespawnMe
  (Utilities|Time|ClearandInvalidateTimerbyHandle (Variables|FlagsAndStuff|GetrespawnTimer))
  (Rendering|SetVisibility (Variables|Default|GethealthPickupSmall) true false)
  (Variables|flagsandstuff|SetisActive true)
  (return))

(fn TryActivatingMe
  (params (overlappingCharacter :type BP%20FPS%20Base%20Character%20Object%20Reference))
  ;[1 1 1] Can health be picked up?
  (if (Math|Boolean|ANDBoolean (Variables|flagsandstuff|GetisActive) (< (Variables|/Game/NewStreak/Core/Characters/BP_FPSBaseCharacter.BP_FPSBaseCharacter_C|GetHealth overlappingCharacter) (Variables|/Game/NewStreak/Core/Characters/BP_FPSBaseCharacter.BP_FPSBaseCharacter_C|GetMaxHealth overlappingCharacter)) (> (Variables|/Game/NewStreak/Core/Characters/BP_FPSBaseCharacter.BP_FPSBaseCharacter_C|GetHealth overlappingCharacter) 0.0))
    ;[1 1 1] give health and play sound/particle effects
    (Networking|SwitchHasAuthority
      (:Authority
        (Default|HealthPickUp overlappingCharacter (Variables|ConfigVariables|GethealAmount) (Variables|ConfigVariables|GetHealSound) (Variables|ConfigVariables|GetHealVFX) (Transformation|GetWorldLocation (Variables|Default|GethealthPickupSmall)))
        ;[1 1 1] deactivate pickup, and hide the health pack part
        (Rendering|SetVisibility (Variables|Default|GethealthPickupSmall) false false)
        (Variables|flagsandstuff|SetisActive false)
        ;[1 1 1] set up delayed respawn
        (bind _returnvalue (Utilities|Time|SetTimerbyFunctionName 0 "respawnMe" (Variables|ConfigVariables|GetrespawnDelay)))
        (Variables|FlagsAndStuff|SetrespawnTimer _returnvalue)
        (return)))))

(fn RotationAnimation
  (Transformation|AddLocalRotation (Variables|Default|GethealthPickupSmall) "0,1.750000, 0" false false)
  (Transformation|AddLocalRotation (Variables|Default|GetpickupHoverStand) (Math|Rotator|MakeRotator 0.0 0.0 (* (/ (Utilities|Time|GetTimerRemainingTimebyHandle (Variables|FlagsAndStuff|GetrespawnTimer)) (Variables|ConfigVariables|GetrespawnDelay)) -1e+01)) false false) ; spin base during respawn delay
)