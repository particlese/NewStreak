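; BP_deathStation is an environment hazard that damages a BP_FPSBaseCharacter while it overlaps the actor.
; Overlap events forward to handler events, with begin-overlap handling marked as server side, which apply damage on entry and start a looping timer.
; The timer reapplies damage at a set interval until a character leaves and clears it.
; Only one character reference and timer handle are stored, so each new entrant overwrites them.
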(event Custom|Event%20EndOverlapHandler
  (params (Leaving%20Actor :type Actor%20Object%20Reference))
  ;[1 1 1] server side
  (Utilities|Casting|CastToBP_FPSBaseCharacter Leaving%20Actor)
  (Utilities|Time|ClearandInvalidateTimerbyHandle (Variables|Default|GetactivationChecker)))

(event Custom|TryToActivate
  ;[1 1 1] server side
  ;;[1 1 1] keep checking until endOverlap triggers
  (Game|Damage|ApplyDamage (stale Custom|Event%20BeginOverlapHandler _asbp_fpsbase_character) (Variables|Default|GetdamageAmount) 0 0))

(event Custom|Event%20BeginOverlapHandler
  (params (OverlappingActor :type Actor%20Object%20Reference))
  ;[1 1 1] server side
  (bind _asbp_fpsbase_character (Utilities|Casting|CastToBP_FPSBaseCharacter OverlappingActor))
  (Game|Damage|ApplyDamage 0 (Variables|Default|GetdamageAmount) 0 0)
  ;;[1 1 1] keep checking until endOverlap triggers
  (bind _returnvalue (Utilities|Time|SetTimerbyEvent (delegate Custom|TryToActivate) (Variables|Default|GetactivationCheckerInterval) true))
  (Variables|Default|SetactivationChecker _returnvalue))

(event Collision|EventActorEndOverlap
  (params (OtherActor :type Actor%20Object%20Reference))
  ;[1 1 1] client
  (CallFunction|EventEndOverlapHandler OtherActor))

(event Collision|EventActorBeginOverlap
  (params (OtherActor :type Actor%20Object%20Reference))
  ;[1 1 1] client
  (CallFunction|EventBeginOverlapHandler OtherActor))

(fn ConstructionScript)