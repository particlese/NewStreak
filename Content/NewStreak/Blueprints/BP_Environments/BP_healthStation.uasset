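; BP_healthStation is a health station that heals player characters while they overlap it.
; Overlap by a BP_FPSBaseCharacter triggers an immediate GiveHealth and starts a looping timer that retries until the character leaves.
; GiveHealth requires a living, injured character and, only on authority, calls its HealthPickUp with heal amount, sound, VFX and station location.
; It tracks one character and one timer handle, so a new overlap overwrites both.
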(event Custom|Event%20EndOverlapHandler
  (params (Leaving%20Actor :type Actor%20Object%20Reference))
  ;[1 1 1] server side
  (Utilities|Casting|CastToBP_FPSBaseCharacter Leaving%20Actor)
  (Utilities|Time|ClearandInvalidateTimerbyHandle (Variables|Default|GetactivationChecker)))

(event Custom|TryToActivate
  ;[1 1 1] server side
  ;;[1 1 1] keep checking until endOverlap triggers
  (CallFunction|GiveHealth (stale Custom|Event%20BeginOverlapHandler _asbp_fpsbase_character)))

(event Custom|Event%20BeginOverlapHandler
  (params (OverlappingActor :type Actor%20Object%20Reference))
  ;[1 1 1] server side
  (bind _asbp_fpsbase_character (Utilities|Casting|CastToBP_FPSBaseCharacter OverlappingActor))
  (CallFunction|GiveHealth _asbp_fpsbase_character)
  ;;[1 1 1] keep checking until endOverlap triggers
  (bind _returnvalue (Utilities|Time|SetTimerbyEvent (delegate Custom|TryToActivate) (Variables|Default|GetactivationCheckerInterval) true))
  (Variables|Default|SetactivationChecker _returnvalue))

(event Collision|EventActorEndOverlap
  (params (OtherActor :type Actor%20Object%20Reference))
  ;[1 1 1] client
  (CallFunction|EventEndOverlapHandler OtherActor))

(event Collision|EventActorBeginOverlap
  (params (OtherActor :type Actor%20Object%20Reference))
  ;[1 1 1] client
  (CallFunction|EventBeginOverlapHandler OtherActor))

(fn ConstructionScript)

(fn GiveHealth
  (params (overlappingCharacter :type BP%20FPS%20Base%20Character%20Object%20Reference))
  ;[1 1 1] Can health be picked up?
  (if (and (< (Variables|/Game/NewStreak/Core/Characters/BP_FPSBaseCharacter.BP_FPSBaseCharacter_C|GetHealth overlappingCharacter) (Variables|/Game/NewStreak/Core/Characters/BP_FPSBaseCharacter.BP_FPSBaseCharacter_C|GetMaxHealth overlappingCharacter)) (> (Variables|/Game/NewStreak/Core/Characters/BP_FPSBaseCharacter.BP_FPSBaseCharacter_C|GetHealth overlappingCharacter) 0.0))
    ;[1 1 1] give health and play sound/particle effects
    (Networking|SwitchHasAuthority
      (:Authority
        (Default|HealthPickUp overlappingCharacter (Variables|Default|GethealAmount) (Variables|Default|GethealSound) (Variables|Default|GetHealVFX) (Transformation|GetWorldLocation (Variables|Default|Getstation)))))))