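; Wraith player character Blueprint with double jump, a timed impulse slide and wall running on tagged walls.
; Holding Space on a wall zeroes gravity, locks height with a plane constraint and pushes along the camera direction captured at contact.
; Left and right detectors drive timelines that roll the control rotation while airborne.
; Landing or wall contact resets the jump count; the wall-run fuel check is defined but never called here.
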(event OnComponentBeginOverlap(RightDetector)
  (params (OverlappedComponent :type Primitive%20Component%20Object%20Reference) (OtherActor :type Actor%20Object%20Reference) (OtherComp :type Primitive%20Component%20Object%20Reference) (OtherBodyIndex :type Integer) (bFromSweep :type Boolean) (SweepResult :type Hit%20Result%20Structure%20%28by%20ref%29))
  ;[1 1 1] RightDetector
  (if (and (Actor|ActorHasTag OtherActor "Runwall") (AI|Components|NavMovement|IsFalling (Variables|Character|GetCharacterMovement)))
    (bind _newtrack_0 (Timeline|Timeline_3 PlayFromStart)
      (:Update
        (Variables|Default|SetTrackRight _newtrack_0)
        (CallFunction|SetRightRotator)))))

(event OnComponentBeginOverlap(LeftDetector)
  (params (OverlappedComponent :type Primitive%20Component%20Object%20Reference) (OtherActor :type Actor%20Object%20Reference) (OtherComp :type Primitive%20Component%20Object%20Reference) (OtherBodyIndex :type Integer) (bFromSweep :type Boolean) (SweepResult :type Hit%20Result%20Structure%20%28by%20ref%29))
  ;[1 1 1] LeftDetector
  (if (and (AI|Components|NavMovement|IsFalling (Variables|Character|GetCharacterMovement)) (Actor|ActorHasTag OtherActor "Runwall"))
    (bind _newtrack_0 (Timeline|Timeline_0 PlayFromStart)
      (:Update
        (Variables|Default|SetTrackLeft _newtrack_0)
        (CallFunction|SetLeftRotator)))))

(event OnComponentBeginOverlap(WallDetection)
  (params (OverlappedComponent :type Primitive%20Component%20Object%20Reference) (OtherActor :type Actor%20Object%20Reference) (OtherComp :type Primitive%20Component%20Object%20Reference) (OtherBodyIndex :type Integer) (bFromSweep :type Boolean) (SweepResult :type Hit%20Result%20Structure%20%28by%20ref%29))
  ;[1 1 1] WallRunning
  (Utilities|FlowControl|Sequence
    (:then_0
      (Utilities|FlowControl|DoN 2) ; enters at Reset
    )
    (:then_1
      (if (Variables|Default|GetCanWallRun)
        (Utilities|FlowControl|Sequence
          (:then_0
            (CallFunction|PlayerDirction)
            (if (and (Actor|ActorHasTag OtherActor "RunWall") (AI|Components|NavMovement|IsFalling (Variables|Character|GetCharacterMovement)))
              (Variables|Default|SetOnWall true)
              (Timeline|Timeline_2 Play
                (:Update
                  (if (> (Class|PlayerController|GetInputKeyTimeDown (Game|GetPlayerController 0) "SpaceBar") 0.0)
                    (if (Variables|Default|GetOnWall)
                      (CallFunction|WallRunStart)
                      (else
                        (CallFunction|WallRunStop)))
                    (else
                      (CallFunction|ResetRotation)))))))
          (:then_1
            (CallFunction|SetPreRotation)))))))

(event OnComponentEndOverlap(WallDetection)
  (params (OverlappedComponent :type Primitive%20Component%20Object%20Reference) (OtherActor :type Actor%20Object%20Reference) (OtherComp :type Primitive%20Component%20Object%20Reference) (OtherBodyIndex :type Integer))
  ;[1 1 1] WallRunning
  (Utilities|FlowControl|Sequence
    (:then_0
      (Timeline|Timeline_2 Stop
        (:Update
          (if (> (Class|PlayerController|GetInputKeyTimeDown (Game|GetPlayerController 0) "SpaceBar") 0.0)
            (if (Variables|Default|GetOnWall)
              (CallFunction|WallRunStart)
              (else
                (CallFunction|WallRunStop :!label _label)))
            (else
              (CallFunction|ResetRotation))))))
    (:then_1
      (if (Actor|ActorHasTag OtherActor "RunWall")
        (goto _label)))))

(event OnComponentEndOverlap(RightDetector)
  (params (OverlappedComponent :type Primitive%20Component%20Object%20Reference) (OtherActor :type Actor%20Object%20Reference) (OtherComp :type Primitive%20Component%20Object%20Reference) (OtherBodyIndex :type Integer))
  ;[1 1 1] RightDetector
  (if (and (Actor|ActorHasTag (stale OnComponentBeginOverlap(RightDetector) OtherActor) "Runwall") (AI|Components|NavMovement|IsFalling (Variables|Character|GetCharacterMovement)))
    (bind _newtrack_0 (Timeline|Timeline_3 ReverseFromEnd)
      (:Update
        (Variables|Default|SetTrackRight _newtrack_0)
        (CallFunction|SetRightRotator)))))

(event OnComponentEndOverlap(LeftDetector)
  (params (OverlappedComponent :type Primitive%20Component%20Object%20Reference) (OtherActor :type Actor%20Object%20Reference) (OtherComp :type Primitive%20Component%20Object%20Reference) (OtherBodyIndex :type Integer))
  ;[1 1 1] LeftDetector
  (if (and (AI|Components|NavMovement|IsFalling (Variables|Character|GetCharacterMovement)) (Actor|ActorHasTag (stale OnComponentBeginOverlap(LeftDetector) OtherActor) "Runwall"))
    (bind _newtrack_0 (Timeline|Timeline_0 ReverseFromEnd)
      (:Update
        (Variables|Default|SetTrackLeft _newtrack_0)
        (CallFunction|SetLeftRotator)))))

(event EventOnLanded
  (params (Hit :type Hit%20Result%20Structure%20%28by%20ref%29))
  ;[1 1 1] WallRunning
  (Utilities|FlowControl|DoN 2) ; enters at Reset
)

(event EventBeginPlay
  ;[1 1 1] BeginPlay
  (Class|MovementComponent|SetPlaneConstraintEnabled (Variables|Character|GetCharacterMovement) true)
  (Variables|Default|SetWallRunFuel 3.3))

(event Input|ActionEvents|InputActionMoveAbility
  (params (Key :type Key%20Structure))
  ;[1 1 1] MoveAbility
  (:Pressed
    (CallFunction|SetDefaultVelocity)
    (CallFunction|RotateIntoSlide)
    (CallFunction|SlideImpulse)
    (Utilities|FlowControl|Delay 0.5)
    (CallFunction|RotatefromSlide)
    (CallFunction|ResetVelocity)))

(event Input|ActionEvents|InputActionJump
  (params (Key :type Key%20Structure))
  ;[1 1 1] WallRunning
  (:Pressed
    (bind _counter (Utilities|FlowControl|DoN 2)
      (:Exit
        (switch int _counter
          (:1
            _)
          (:2
            _))
        (Character|LaunchCharacter "0, 0,400.000000" false true))))
  (:Released
    (Character|StopJumping)))

(fn ConstructionScript)

(fn SetRightRotator
  (bind _returnvalue (Transformation|GetActorRotation))
  (bind (_roll _pitch _yaw) (Math|Rotator|BreakRotator _returnvalue))
  (Pawn|SetControlRotation (Game|GetPlayerController 0) (Math|Rotator|Lerp(Rotator) _returnvalue (Math|Rotator|MakeRotator -2e+01 _pitch _yaw) (Variables|Default|GetTrackRight))))

(fn SetLeftRotator
  (bind _returnvalue (Transformation|GetActorRotation))
  (bind (_roll _pitch _yaw) (Math|Rotator|BreakRotator _returnvalue))
  (Pawn|SetControlRotation (Game|GetPlayerController 0) (Math|Rotator|Lerp(Rotator) _returnvalue (Math|Rotator|MakeRotator 2e+01 _pitch _yaw) (Variables|Default|GetTrackLeft))))

(fn SlideImpulse
  (bind _camera (Variables|Default|GetCamera))
  (bind _returnvalue (Math|Vector|GetForwardVector _camera))
  (Physics|AddImpulse (Variables|Character|GetCharacterMovement) (* (Math|Vector|MakeVector (.x _returnvalue) (.y _returnvalue) 0.0) (* (Input|AxisValues|GetMoveForward) 4e+03)) true))

(fn RotateIntoSlide
  (bind _mesh (Variables|Character|GetMesh))
  (bind _relativerotation (Variables|/Script/Engine.SceneComponent|GetRelativeRotation _mesh))
  (Transformation|SetRelativeRotation _mesh (Math|Rotator|MakeRotator -9e+01 (.pitch _relativerotation) (.yaw _relativerotation)) false false))

(fn RotatefromSlide
  (bind _mesh (Variables|Character|GetMesh))
  (bind _relativerotation (Variables|/Script/Engine.SceneComponent|GetRelativeRotation _mesh))
  (Transformation|SetRelativeRotation _mesh (Math|Rotator|MakeRotator 0.0 (.pitch _relativerotation) (.yaw _relativerotation)) false false))

(fn WallRunStop
  (bind _charactermovement (Variables|Character|GetCharacterMovement))
  (Variables|/Script/Engine.CharacterMovementComponent|SetGravityScale _charactermovement 1.0)
  (Class|MovementComponent|SetPlaneConstraintNormal _charactermovement "0, 0, 0")
  (Variables|Default|SetOnWall false))

(fn WallRunStart
  (bind _charactermovement (Variables|Character|GetCharacterMovement))
  (Variables|/Script/Engine.CharacterMovementComponent|SetGravityScale _charactermovement 0.0)
  (Class|MovementComponent|SetPlaneConstraintNormal _charactermovement "0, 0,1.000000")
  (Physics|AddForce _charactermovement (Variables|Default|GetPlayerDirection)))

(fn ResetRotation
  (Pawn|SetControlRotation (Game|GetPlayerController 0) (Variables|Default|GetPreRotation)))

(fn SetPreRotation
  (Variables|Default|SetPreRotation (Transformation|GetActorRotation (Game|GetPlayerController 0))))

(fn PlayerDirction
  (Variables|Default|SetPlayerDirection (Math|Vector|GetForwardVector (Variables|Default|GetCamera))))

(fn PrintonScreen
  (Development|PrintString (Utilities|String|ToString(Float) (Variables|Default|GetWallRunFuel))))

(fn CheckFuel
  (Variables|Default|SetCanWallRun (<= (Class|PlayerController|GetInputKeyTimeDown (Game|GetPlayerController 0) "SpaceBar") (Variables|Default|GetWallRunFuel))))