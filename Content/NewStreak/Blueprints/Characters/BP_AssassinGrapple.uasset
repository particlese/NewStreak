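; BP_AssassinGrapple is a grapple actor with an anchor and a stretched cable mesh linking it to its Instigator, apparently the assassin player.
; Each tick scales the Cable to the separation distance, centers it at the midpoint and aligns it along that vector with a 90-degree offset.
; The embedinsurface event orients the Anchor from the supplied surface normal.
; The actor destroys itself when the Instigator is destroyed.
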(event OnDestroyed(Instigator)
  (params (DestroyedActor :type Actor%20Object%20Reference))
  (Actor|DestroyActor))

(event Custom|embed%20in%20surface
  (params (embedNormal :type Vector))
  ;[1 1 1] rotate anchor
  (Transformation|SetRelativeRotation (Variables|Default|Getanchor) (Math|Rotator|CombineRotators "90.000000, 0,0.000000" (Math|Conversions|RotationFromXVector embedNormal)) false false))

(event EventBeginPlay)

(event Collision|EventActorBeginOverlap
  (params (OtherActor :type Actor%20Object%20Reference)))

(event EventTick
  (params (DeltaSeconds :type Float%20%28single-precision%29))
  (bind _returnvalue (Transformation|GetActorLocation))
  (bind _instigator (Variables|Actor|GetInstigator))
  (bind _returnvalue_2 (Transformation|GetActorLocation _instigator))
  (bind _returnvalue_3 (- _returnvalue _returnvalue_2))
  ;[1 1 1] adjust cable
  (Utilities|FlowControl|Sequence
    (:then_0
      (Transformation|SetWorldScale3D (Variables|Default|Getcable) (Math|Vector|MakeVector 0.05 0.05 (/ (Math|Vector|VectorLength _returnvalue_3) 1e+02))))
    (:then_1
      (Transformation|SetWorldLocationAndRotation (Variables|Default|Getcable) (* (+ _returnvalue _returnvalue_2) 0.5) (Math|Rotator|FindLookatRotation _returnvalue_2 _returnvalue) false false))
    (:then_2
      (Transformation|SetRelativeRotation (Variables|Default|Getcable) (Math|Rotator|CombineRotators "90.000000, 0, 0" (Math|Conversions|RotationFromXVector _returnvalue_3)) false false))))

(fn ConstructionScript)