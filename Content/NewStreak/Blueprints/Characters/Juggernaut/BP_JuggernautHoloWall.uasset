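; BP_JuggernautHoloWall is the Juggernaut character's holographic wall, a damageable actor that animates in and out.
; On BeginPlay it caches the Wall component's scale, then a timeline scales it up to that deployed size.
; Damage lowers Health on the authority only, calling for destruction at zero.
; The guarded destroy event disables collision, plays a shrink timeline relative to the cached scale, then destroys the actor.
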(event Custom|Event%20destroyWall
  ;[1 1 1] destruction/removal
  (if (not (Variables|Default|GetdestructionInProgress))
    (Variables|Default|SetdestructionInProgress true)
    (Collision|SetActorEnableCollision false)
    (bind _scale (Timeline|wallShrink PlayFromStart)
      (:Update
        (Transformation|SetRelativeScale3D (Variables|Default|Getwall) (* (Math|Conversions|ToVector(Float) _scale) (Variables|Default|GetdeployedScale))))
      (:Finished
        (Actor|DestroyActor)))))

(event EventBeginPlay
  ;[1 1 1] adapt destruction shrinkage-on-destroy to however it's set up in the viewport tab over there
  (Variables|Default|SetdeployedScale (.Scale (Math|Transform|BreakTransform (Transformation|GetRelativeTransform (Variables|Default|Getwall)))))
  ;[1 1 1] deployment animation
  (bind _scale (Timeline|wallDeploy PlayFromStart)
    (:Update
      (Transformation|SetRelativeScale3D (Variables|Default|Getwall) (* (Math|Conversions|ToVector(Float) _scale) (Variables|Default|GetdeployedScale))))))

(event Game|Damage|EventAnyDamage
  (params (Damage :type Float%20%28single-precision%29) (DamageType :type Damage%20Type%20Object%20Reference) (InstigatedBy :type Controller%20Object%20Reference) (DamageCauser :type Actor%20Object%20Reference))
  ;[1 1 1] take damage
  (Networking|SwitchHasAuthority
    (:Authority
      (bind _output_get (Variables|Default|SetHealth (- (Variables|Default|GetHealth) Damage)))
      (if (<= _output_get 0.0)
        (CallFunction|EventDestroyWall)))))

(fn ConstructionScript)