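; BP_Harrier is a first-person playable character with aerial movement: double jump, laser kick and laser boots.
; Jumps launch vertically through a DoN gate reset on landing, and the kick checks fuel before launching opposite the camera's forward vector.
; While the ability is held, Tick applies camera-relative boot thrust, redirected backward on reverse input, with quadratic drag as a soft speed limit.
; BeginPlay adds a fuel widget.
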(event EventBeginPlay
  ;[1 1 1] BeginPlay
  (|CallParentFunction)
  (bind _returnvalue (UserInterface|CreateWidget "/Game/NewStreak/Core/CoreUIandEffects/BP_Fuel.BP_Fuel_C"))
  (UserInterface|Viewport|AddtoViewport _returnvalue 0))

(event EventTick
  (params (DeltaSeconds :type Float%20%28single-precision%29))
  (bind _returnvalue (Transformation|GetVelocity))
  (bind _firstpersoncamera (Variables|Default|GetFirstPersonCamera))
  (bind _charactermovement (Variables|Character|GetCharacterMovement))
  (bind _returnvalue_2 (Math|Vector|VectorLength _returnvalue))
  (bind _returnvalue_3 (Math|Vector|Normalize _returnvalue))
  (bind _returnvalue_4 (* _returnvalue_2 _returnvalue_2 0.05))
  (bind _returnvalue_5 (* _returnvalue_3 _returnvalue_4))
  ;[1 1 1] Laser boots (shift key ability)
  (if (Variables|Default|GetlaserBootsOn)
    (if (< (Input|AxisValues|GetMoveForward) 0.0)
      (Physics|AddForce _charactermovement (- (* (Math|Vector|GetForwardVector (Variables|Default|GetFirstPersonCamera)) (* (Variables|Default|GetlaserBootsThrust) (Physics|GetMass (Variables|Default|GetCapsuleComponent)) -1.0)) _returnvalue_5))
      (else
        (Physics|AddForce _charactermovement (- (* (Math|Vector|RotateVectorAroundAxis (Math|Vector|GetForwardVector _firstpersoncamera) -9e+01 (Math|Vector|GetRightVector _firstpersoncamera)) (* (Variables|Default|GetlaserBootsThrust) (Physics|GetMass (Variables|Default|GetCapsuleComponent)))) _returnvalue_5))))))

(event EventOnLanded
  (params (Hit :type Hit%20Result%20Structure%20%28by%20ref%29))
  ;[1 1 1] Jump (double)
  ;;[1 1 1] jump debugging stuff
  (if (Variables|Default|GetprintDebugOutput)
    (CallFunction|PrintJumpDuration)
    (Utilities|FlowControl|DoN 2) ; enters at Reset
    (else
      (Utilities|FlowControl|DoN 2) ; enters at Reset
    )))

(event Input|ActionEvents|InputActionJump
  (params (Key :type Key%20Structure))
  ;[1 1 1] Jump (double)
  (:Pressed
    (bind _counter (Utilities|FlowControl|DoN 2)
      (:Exit
        (switch int _counter
          (:1
            _)
          (:2
            _))
        (bind _launchvector (CallFunction|GetZLaunchfromJumpDuration 0.75))
        (Character|LaunchCharacter _launchvector false true)
        ;;[1 1 1] jump debugging stuff
        (CallFunction|PrintJumpLaunchImpulse _launchvector)
        (CallFunction|SetJumpStartTime)))))

(event Input|ActionEvents|InputActionKick
  (params (Key :type Key%20Structure))
  ;[1 1 1] laser kick
  (:Pressed
    (if (>= (Variables|Default|GetFuel) (Variables|Default|GetlaserKickFuelUse))
      (Character|LaunchCharacter (* (Math|Vector|GetForwardVector (Variables|Default|GetFirstPersonCamera)) -1.2e+03) true true))))

(event Input|ActionEvents|InputActionMoveAbility
  (params (Key :type Key%20Structure))
  ;[1 1 1] Laser boots (shift key ability)
  ;;[1 1 1] Toggle
  (:Pressed
    (Variables|Default|SetlaserBootsOn true))
  (:Released
    (Variables|Default|SetlaserBootsOn false)))

(fn ConstructionScript
  (|CallParentFunction))

(fn PrintJumpDuration
  (Development|PrintString (Utilities|String|Append "Landed " (Utilities|String|ToString(Float) (- (Utilities|Time|GetGameTimeinSeconds) (Variables|Default|GetjumpStartTime))) " seconds after last jump.")))

(fn SetJumpStartTime
  (Variables|Default|SetjumpStartTime (Utilities|Time|GetGameTimeinSeconds)))

(fn PrintJumpLaunchImpulse
  (params (launchImpulse :type Vector))
  (CallFunction|SetJumpStartTime)
  (if (Variables|Default|GetprintDebugOutput)
    (Development|PrintString (Utilities|String|Append "Launched at " (Utilities|String|ToString(Float) (.Z (Math|Vector|BreakVector launchImpulse))) " cm/s or whatever."))))

(fn GetFPCamVector
  (bind _firstpersoncamera (Variables|Default|GetFirstPersonCamera))
  (bind _returnvalue (Transformation|GetWorldRotation _firstpersoncamera))
  (bind (_roll _pitch _yaw) (Math|Rotator|BreakRotator _returnvalue))
  (return (Class|KismetMathLibrary|CreateVectorfromYawPitch _yaw _pitch 1.0)))